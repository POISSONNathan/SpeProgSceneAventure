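; Player controller that owns the player's life, mana, gold and spell loadout, pushing changes to the WBP_Interface HUD.
; Bought spells become BP_OnGameSpell objects with Tick-updated cooldowns, selected by R/T/Y/U and cast after cooldown and condition checks.
; Zero life plays the death animation, then respawns the pawn at its starting location after a delay.
; It also forwards interaction input and times long-cast animations that lock movement.
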(event Custom|LongAnimCastSpell
  (params (CurrentSpell :type BP%20DA%20Spell%20Object%20Reference))
  ;[1 0.8438 0.9821] Animation spell
  (Variables|/Game/Blueprints/Player/Character/ABP_AnimMainCharacter.ABP_AnimMainCharacter_C|SetanimCastLongSpell (CallFunction|GetABPas) true)
  (Variables|/Game/Blueprints/Player/ThirdPersonCharacter.ThirdPersonCharacter_C|SetcantMove (CallFunction|GetPlayerCharacteras) true)
  (Utilities|FlowControl|Sequence
    (:then_0
      (Utilities|FlowControl|Delay 2.0)
      (Variables|Default|SetinSpellAnimation false)
      (Variables|/Game/Blueprints/Player/Character/ABP_AnimMainCharacter.ABP_AnimMainCharacter_C|SetanimCastLongSpell (CallFunction|GetABPas) false)
      (Variables|/Game/Blueprints/Player/ThirdPersonCharacter.ThirdPersonCharacter_C|SetcantMove (CallFunction|GetPlayerCharacteras) false))
    (:then_1
      (Utilities|FlowControl|Delay 1.0)
      (Default|Action CurrentSpell self (CallFunction|GetPlayerCharacteras)))))

(event Custom|ResetVariable
  ;[0.7703 1 0.7232] Reset all stats
  (Variables|Default|Setlife (Variables|Default|GetmaxLife))
  (Variables|Default|Setmana (Variables|Default|GetmanaMax))
  (Variables|Default|Setgold 0)
  (Utilities|FlowControl|Sequence
    (:then_0
      (CallFunction|SetLife 0.0))
    (:then_1
      (CallFunction|SetMana 0.0))
    (:then_2
      (CallFunction|SetGold))))

(event Custom|Respawn
  ;[1 0.9898 0.7891] Respawn at 1st position
  (Transformation|SetActorLocation (Game|Player|GetPlayerPawn 0) (Variables|Default|GetrespawnPoint) false false)
  (Variables|/Game/Blueprints/Player/Character/ABP_AnimMainCharacter.ABP_AnimMainCharacter_C|SetisDead (CallFunction|GetABPas) false)
  (Input|EnableInput (CallFunction|GetPlayerCharacteras) 0))

(event Custom|AnimDead
  ;[1 0.9898 0.7891] Respawn at 1st position
  (Variables|/Game/Blueprints/Player/Character/ABP_AnimMainCharacter.ABP_AnimMainCharacter_C|SetisDead (CallFunction|GetABPas) true)
  (Input|DisableInput (CallFunction|GetPlayerCharacteras) 0)
  (Utilities|FlowControl|Delay 3.0)
  (CallFunction|Respawn))

(event Custom|UpdateSelectedSpell
  (params (indexSpellInList :type Integer) (Target :type WBP%20Interface%20Object%20Reference))
  (bind _myui (Variables|Default|GetmyUi))
  ;[1 0.8245 0.6691] Spells (switch and cast) + Cooldown
  (if (Utilities|IsValid (Utilities|Array|Get(acopy) (Variables|Default|GetcurrentSpells) indexSpellInList))
    (Default|MoveSelectedSpell _myui (Widget|GetParent (Utilities|Array|Get(acopy) (Variables|/Game/Blueprints/Player/WBP_Interface.WBP_Interface_C|GetlistImageInventory _myui) indexSpellInList)))))

(event EventBeginPlay
  ;[1 0.6463 0.7266] Start
  (bind _returnvalue (UserInterface|CreateWidget "/Game/Blueprints/Player/WBP_Interface.WBP_Interface_C"))
  (bind _output_get (Variables|Default|SetmyUi _returnvalue))
  (UserInterface|Viewport|AddtoViewport _output_get 0)
  (CallFunction|ResetVariable)
  (Variables|Default|SetrespawnPoint (Transformation|GetActorLocation (Game|Player|GetPlayerPawn 0)))
  (Default|SetInventory (Variables|Default|GetmyUi)))

(event EventTick
  (params (DeltaSeconds :type Float%20%28single-precision%29))
  ;[1 0.8245 0.6691] Spells (switch and cast) + Cooldown
  (for _array_element (Variables|Default|GetcurrentSpells)
    (Default|UpdateCooldown _array_element DeltaSeconds)))

(event Input|ActionEvents|InputActionInteractionButton
  (params (Key :type Key%20Structure :default "None"))
  ;[0.7065 0.8656 1] Interact
  (:Pressed
    (bind _myinteractable (Variables|Default|GetmyInteractable)
      (:then
        (Default|InteractwithObj _myinteractable))
      (:else))))

(event Input|ActionEvents|InputActionCastSpellButton
  (params (Key :type Key%20Structure :default "None"))
  (bind _output (CallFunction|GetCurrentSpell))
  (bind _output_2 (CallFunction|GetCurrentSpell))
  ;[1 0.8245 0.6691] Spells (switch and cast) + Cooldown
  (:Pressed
    (Utilities|IsValid _output
      (:Is%20Valid
        (if (Variables|/Game/Blueprints/Spell/BP_OnGameSpell.BP_OnGameSpell_C|GetCanCast _output)
          (if (Default|ConditiontoCast (Variables|/Game/Blueprints/Spell/BP_OnGameSpell.BP_OnGameSpell_C|GetSpell _output) (CallFunction|GetPlayerControlleras) (CallFunction|GetPlayerCharacteras))
            (Default|AdditionalEffect (Variables|/Game/Blueprints/Spell/BP_OnGameSpell.BP_OnGameSpell_C|GetSpell (CallFunction|GetCurrentSpell)) self (CallFunction|GetPlayerCharacteras))
            (CallFunction|SetMana (* (Variables|/Game/Blueprints/Spell/BP_DA_Spell.BP_DA_Spell_C|GetManaCost (Variables|/Game/Blueprints/Spell/BP_OnGameSpell.BP_OnGameSpell_C|GetSpell _output_2)) -1.0))
            (Variables|/Game/Blueprints/Spell/BP_OnGameSpell.BP_OnGameSpell_C|SetCanCast _output_2 false)
            (Default|ResetCooldown _output_2)))))))

(event Input|KeyboardEvents|U
  (params (Key :type Key%20Structure :default "None"))
  ;[1 0.8245 0.6691] Spells (switch and cast) + Cooldown
  (:Pressed
    (if (not (Variables|Default|GetinSpellAnimation))
      (bind _output_get (Variables|Default|SetCurrentSpellIndex 3))
      (CallFunction|UpdateSelectedSpell _output_get (Variables|Default|GetmyUi)))))

(event Input|KeyboardEvents|R
  (params (Key :type Key%20Structure :default "None"))
  ;[1 0.8245 0.6691] Spells (switch and cast) + Cooldown
  (:Pressed
    (if (not (Variables|Default|GetinSpellAnimation))
      (bind _output_get (Variables|Default|SetCurrentSpellIndex 0))
      (CallFunction|UpdateSelectedSpell _output_get (Variables|Default|GetmyUi)))))

(event Input|KeyboardEvents|Y
  (params (Key :type Key%20Structure :default "None"))
  ;[1 0.8245 0.6691] Spells (switch and cast) + Cooldown
  (:Pressed
    (if (not (Variables|Default|GetinSpellAnimation))
      (bind _output_get (Variables|Default|SetCurrentSpellIndex 2))
      (CallFunction|UpdateSelectedSpell _output_get (Variables|Default|GetmyUi)))))

(event Input|KeyboardEvents|T
  (params (Key :type Key%20Structure :default "None"))
  ;[1 0.8245 0.6691] Spells (switch and cast) + Cooldown
  (:Pressed
    (if (not (Variables|Default|GetinSpellAnimation))
      (bind _output_get (Variables|Default|SetCurrentSpellIndex 1))
      (CallFunction|UpdateSelectedSpell _output_get (Variables|Default|GetmyUi)))))

(fn ConstructionScript)

(fn SetLife
  (params (AmmountOfLife :type Float%20%28single-precision%29))
  (bind _myui (Variables|Default|GetmyUi))
  (Variables|Default|Setlife (Math|Float|ClampAngle (+ (Variables|Default|Getlife) AmmountOfLife) 0.0 (Variables|Default|GetmaxLife)))
  (Default|SetUIStat _myui (Variables|/Game/Blueprints/Player/WBP_Interface.WBP_Interface_C|GetLifeBar _myui) (/ (Variables|Default|Getlife) (Variables|Default|GetmaxLife)))
  (if (<= (Variables|Default|Getlife) 0.0)
    (CallFunction|AnimDead)))

(fn SetMana
  (params (AmmountOfMana :type Float%20%28single-precision%29))
  (bind _myui (Variables|Default|GetmyUi))
  (Variables|Default|Setmana (Math|Float|ClampAngle (+ (Variables|Default|Getmana) AmmountOfMana) 0.0 (Variables|Default|GetmanaMax)))
  (Default|SetUIStat _myui (Variables|/Game/Blueprints/Player/WBP_Interface.WBP_Interface_C|GetManaBar _myui) (/ (Variables|Default|Getmana) (Variables|Default|GetmanaMax))))

(fn SetGold
  (params (AmmountOfGold :type Integer))
  (Variables|Default|Setgold (Math|Integer|Clamp(Integer) (+ (Variables|Default|Getgold) AmmountOfGold) 0 2147483647))
  (Default|SetUiGold (Variables|Default|GetmyUi) (Utilities|Text|ToText(Integer) (Variables|Default|Getgold))))

(fn SpawnActor
  (params (CurrentActorToSpawn :type Actor%20Class%20Reference) (LocationTransofrm :type Transform))
  (bind _returnvalue (Game|SpawnActorfromClass CurrentActorToSpawn LocationTransofrm "Undefined" 0 0))
  (return _returnvalue))

(fn AddSpell
  (params (CurrentSpellToGive :type BP%20DA%20Spell%20Object%20Reference))
  (if (>= (Variables|Default|Getgold) (Variables|/Game/Blueprints/Spell/BP_DA_Spell.BP_DA_Spell_C|GetGoldCost CurrentSpellToGive))
    (if (or (>= (Utilities|Array|Length (Variables|Default|GetcurrentSpells)) (Variables|Default|GetnumberSpellMax)) (CallFunction|ContainsSpell CurrentSpellToGive))
      (return false)
      (else
        (CallFunction|SetGold (* (Variables|/Game/Blueprints/Spell/BP_DA_Spell.BP_DA_Spell_C|GetGoldCost CurrentSpellToGive) -1))
        (Default|UiSpell (Variables|BP_PlayerController_C|GetmyUi (CallFunction|GetPlayerControlleras)) CurrentSpellToGive)
        (bind _returnvalue (Game|ConstructObjectfromClass "/Game/Blueprints/Spell/BP_OnGameSpell.BP_OnGameSpell_C" self CurrentSpellToGive))
        (bind _output_get (Variables|/Game/Blueprints/Spell/BP_OnGameSpell.BP_OnGameSpell_C|SetprogressBarUI _returnvalue (Utilities|Array|Get(acopy) (Variables|/Game/Blueprints/Player/WBP_Interface.WBP_Interface_C|GetlistCooldownBar (Variables|Default|GetmyUi)) (Utilities|Array|Length (Variables|Default|GetcurrentSpells)))))
        (Widget|SetVisibility _output_get "Visible")
        (Variables|/Game/Blueprints/Spell/BP_OnGameSpell.BP_OnGameSpell_C|SetCanCast _returnvalue true)
        (bind _returnvalue_2 (Utilities|Array|Add (Variables|Default|GetcurrentSpells) _returnvalue))
        (Variables|Default|SetCurrentSpellIndex _returnvalue_2)
        (return true)))))

(fn GetCurrentSpell
  (return (Utilities|Array|Get(acopy) (Variables|Default|GetcurrentSpells) (Variables|Default|GetCurrentSpellIndex))))

(fn ContainsSpell
  (params (SpellToGive :type Object%20Object%20Reference))
  (for _array_element (Variables|Default|GetcurrentSpells)
    (if (== (Variables|/Game/Blueprints/Spell/BP_OnGameSpell.BP_OnGameSpell_C|GetSpell _array_element) SpellToGive)
      (return true)))
  (return false))