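; BP_Enemy is an enemy actor with health and a life bar widget component.
; On BeginPlay it caches the WBP_EnemyLifeBar widget and sets Life to MaxLife.
; ChangeLife subtracts damage, sends the life ratio to the widget and destroys the actor when Life reaches zero or below.
; Each tick it rotates the life bar to face the player character's location.
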(event Custom|ChangeLife
  (params (AmmountOfDammage :type Float%20%28single-precision%29))
  (Variables|Default|Setlife (- (Variables|Default|Getlife) AmmountOfDammage))
  (Default|SetEnemyLifeBar (Variables|Default|GetenemyUI) (/ (Variables|Default|Getlife) (Variables|Default|GetmaxLife)))
  (if (CallFunction|IsDead)
    (Actor|DestroyActor)))

(event EventTick
  (params (DeltaSeconds :type Float%20%28single-precision%29))
  (bind _lifebar (Variables|Default|GetLifeBar))
  (Transformation|SetWorldRotation _lifebar (Math|Rotator|FindLookatRotation (Transformation|GetWorldLocation _lifebar) (Transformation|GetActorLocation (CallFunction|GetPlayerCharacteras))) false false))

(event EventBeginPlay
  (bind _aswbp_enemy_life_bar (Utilities|Casting|CastToWBP_EnemyLifeBar (UserInterface|GetUserWidgetObject (Variables|Default|GetLifeBar))))
  (Variables|Default|SetenemyUI _aswbp_enemy_life_bar)
  (Variables|Default|Setlife (Variables|Default|GetmaxLife)))

(fn ConstructionScript)

(fn IsDead
  (return (<= (Variables|Default|Getlife) 0.0)))