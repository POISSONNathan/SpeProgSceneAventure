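; BP_EnemyMove is an enemy Blueprint that sets up behavior tree AI for itself when play begins.
; After the parent BeginPlay, it casts its controller to AIController, runs BT_EnemyAI and sets up the BB_EnemyAI blackboard.
; It then writes its Target1 and Target2 variables into the target1 and target2 blackboard keys, leaving any behavior using them to the tree.
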(event EventBeginPlay
  (|CallParentFunction)
  (bind _asaicontroller (Utilities|Casting|CastToAIController (Pawn|GetController)))
  (AI|RunBehaviorTree _asaicontroller "/Game/Blueprints/EnemyTrap/Enemy/AIEnemy/BT_EnemyAI.BT_EnemyAI")
  (bind _blackboardcomponent (Class|AIController|UseBlackboard _asaicontroller "/Game/Blueprints/EnemyTrap/Enemy/AIEnemy/BB_EnemyAI.BB_EnemyAI"))
  (Utilities|FlowControl|Sequence
    (:then_0
      (AI|Components|Blackboard|SetValueasObject _blackboardcomponent (Utilities|Name|MakeLiteralName "target1") (Variables|Default|Gettarget1)))
    (:then_1
      (AI|Components|Blackboard|SetValueasObject _blackboardcomponent (Utilities|Name|MakeLiteralName "target2") (Variables|Default|Gettarget2)))))

(fn ConstructionScript
  (|CallParentFunction))