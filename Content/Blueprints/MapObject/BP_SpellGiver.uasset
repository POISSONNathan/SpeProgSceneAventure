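; BP_SpellGiver is a map object that gives the player a configured spell on interaction.
; The construction script fills its price text, name text and sprite from the gold cost, name and icon of SpellToGive.
; InteractwithObj passes that spell to AddSpell on the player controller and spawns an after-buy particle effect at the actor, with no gold check in this graph.
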(event EventInteractwithObj
  (Default|AddSpell (CallFunction|GetPlayerControlleras) (Variables|Default|GetspellToGive))
  (Effects|SpawnEmitteratLocation (Variables|Default|GetparticleSpawnAfterBuy) (Transformation|GetActorLocation) "0, 0,0.000000"))

(fn ConstructionScript
  (Rendering|Components|TextRender|SetText (Variables|Default|GetpriceText) (Utilities|Text|ToText(Integer) (Variables|/Game/Blueprints/Spell/BP_DA_Spell.BP_DA_Spell_C|GetGoldCost (Variables|Default|GetspellToGive))))
  (Rendering|Components|Sprite|SetSprite (Variables|Default|GetPaperSprite) (Variables|/Game/Blueprints/Spell/BP_DA_Spell.BP_DA_Spell_C|GetIcon (Variables|Default|GetspellToGive)))
  (Rendering|Components|TextRender|SetText (Variables|Default|GetnameText) (Utilities|Text|ToText(Name) (Variables|/Game/Blueprints/Spell/BP_DA_Spell.BP_DA_Spell_C|GetName (Variables|Default|GetspellToGive)))))