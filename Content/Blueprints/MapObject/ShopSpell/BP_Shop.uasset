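; BP_Shop is an interactable map object that opens and closes a shop screen for the player.
; On BeginPlay it creates a WBP_ShopUI widget and has it build its list buttons, passing itself in.
; Each interaction toggles the OnShop flag, adding or removing the widget from the viewport while disabling or restoring character input and showing or hiding the mouse cursor.
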(event EventInteractwithObj
  (bind _asplayercontroller (CallFunction|GetPlayerControlleras))
  (bind _asplayercontroller_2 (CallFunction|GetPlayerControlleras))
  (if (Variables|Default|GetonShop)
    (Widget|RemovefromParent (Variables|Default|GetshopUI))
    (Input|EnableInput (CallFunction|GetPlayerCharacteras) _asplayercontroller_2)
    (Variables|Default|SetonShop false)
    (Variables|/Script/Engine.PlayerController|SetbShowMouseCursor _asplayercontroller_2 false)
    (else
      (UserInterface|Viewport|AddtoViewport (Variables|Default|GetshopUI) 0)
      (Input|DisableInput (CallFunction|GetPlayerCharacteras) _asplayercontroller)
      (Variables|Default|SetonShop true)
      (Variables|/Script/Engine.PlayerController|SetbShowMouseCursor _asplayercontroller true))))

(event EventBeginPlay
  (bind _returnvalue (UserInterface|CreateWidget "/Game/Blueprints/MapObject/ShopSpell/WBP_ShopUI.WBP_ShopUI_C"))
  (bind _output_get (Variables|Default|SetshopUI _returnvalue))
  (Default|CreateListButton _output_get self))

(fn ConstructionScript
  (|CallParentFunction))