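; NPC actor that plays a linear dialogue through a WBP_PnjUI widget component, one line per InteractwithObj call.
; The first interaction moves the player character just above the Cylinder component, sets its CantMove flag and shows the first line.
; Each later call advances the Dialogues array, and the call that displays the last line also frees the player and resets the index.
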(event Custom|SetText
  (Default|SetPnjText (Variables|Default|GetPnjUI) (Utilities|Array|Get(acopy) (Variables|Default|GetDialogues) (Variables|Default|GetcurrentDialogues)))
  (Variables|Default|SetcurrentDialogues (+ (Variables|Default|GetcurrentDialogues) 1)))

(event EventBeginPlay
  (bind _aswbp_pnj_ui (Utilities|Casting|CastToWBP_PnjUI (UserInterface|GetUserWidgetObject (Variables|Default|GetWidget))))
  (Variables|Default|SetPnjUI _aswbp_pnj_ui))

(event EventInteractwithObj
  (if (Variables|Default|GetisInteracting)
    (CallFunction|SetText)
    (if (>= (Variables|Default|GetcurrentDialogues) (Utilities|Array|Length (Variables|Default|GetDialogues)))
      (Variables|/Game/Blueprints/ThirdPersonCharacter.ThirdPersonCharacter_C|SetcantMove (Variables|Default|GetmyCharacter) false)
      (Variables|Default|SetisInteracting false)
      (Variables|Default|SetcurrentDialogues 0))
    (else
      (Variables|Default|SetisInteracting true)
      (bind _asthird_person_character (Utilities|Casting|CastToThirdPersonCharacter (Game|GetPlayerCharacter 0)))
      (bind _output_get (Variables|Default|SetmyCharacter _asthird_person_character))
      (Transformation|SetActorRelativeLocation _output_get (+ (Transformation|GetWorldLocation (Variables|Default|GetCylinder)) "0.000000,0.000000,50.000000"))
      (Variables|/Game/Blueprints/ThirdPersonCharacter.ThirdPersonCharacter_C|SetcantMove (Variables|Default|GetmyCharacter) true)
      (CallFunction|SetText))))

(fn ConstructionScript
  (|CallParentFunction))