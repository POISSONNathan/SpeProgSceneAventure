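; BP_OnGameSpell tracks the runtime cooldown state of a single spell.
; ResetCooldown restores the current cooldown to the cooldown value in the spell's Data.
; UpdateCooldown subtracts delta time, clamps the result between zero and that value, and sets CanCast once it reaches zero.
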(fn ResetCooldown
  (Variables|Default|SetCurrentCooldown (Variables|/Game/Blueprints/Spell/BP_DA_Spell.BP_DA_Spell_C|GetCooldown (Variables|Default|Getdata))))

(fn UpdateCooldown
  (params (deltaTime :type Float%20%28single-precision%29))
  (bind _output_get (Variables|Default|SetCurrentCooldown (Math|Float|Clamp(Float) (- (Variables|Default|GetCurrentCooldown) deltaTime) 0.0 (Variables|/Game/Blueprints/Spell/BP_DA_Spell.BP_DA_Spell_C|GetCooldown (Variables|Default|Getdata)))))
  (Variables|Default|SetCanCast (<= _output_get 0.0)))