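; BP_SpellGiver is an interactable spell vendor that sells one configured spell for gold.
; On interaction it checks that the player controller's gold exceeds the price and the spell is not already owned.
; It then deducts the gold, adds the spell to the controller's spell list and passes it to the UI.
; The construction script sets the price text and the sprite from the spell's icon.
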(event EventInteractwithObj
  (params (playerCharacter :type Third%20Person%20Character%20Object%20Reference))
  (bind _spelltogive (Variables|Default|GetspellToGive))
  (bind _asbp_player_controller (Utilities|Casting|CastToBP_PlayerController (Game|GetPlayerController 0)))
  (if (> (Variables|/Game/Blueprints/BP_PlayerController.BP_PlayerController_C|Getgold _asbp_player_controller) (Variables|Default|Getprice))
    (if (not (Utilities|Array|ContainsItem (Variables|/Game/Blueprints/BP_PlayerController.BP_PlayerController_C|GetmyListOfSpell _asbp_player_controller) _spelltogive))
      (Default|ChangeGold _asbp_player_controller (* (Variables|Default|Getprice) -1))
      (Utilities|Array|Add (Variables|/Game/Blueprints/BP_PlayerController.BP_PlayerController_C|GetmyListOfSpell _asbp_player_controller) _spelltogive)
      (Default|UiSpell (Variables|/Game/Blueprints/BP_PlayerController.BP_PlayerController_C|GetmyUi _asbp_player_controller) _spelltogive))))

(fn ConstructionScript
  (Rendering|Components|TextRender|SetText (Variables|Default|GetpriceText) (Utilities|Text|ToText(Integer) (Variables|Default|Getprice)))
  (Rendering|Components|Sprite|SetSprite (Variables|Default|GetPaperSprite) (Variables|/Game/Blueprints/Spell/BP_DA_Spell.BP_DA_Spell_C|GetIcon (Variables|Default|GetspellToGive))))