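; Poison spell asset, apparently a data asset, that throws a poison potion from the casting player character.
; CastSpell runs the parent's cast and fires Action only when that succeeds.
; Action spawns BP_Poison just ahead of the character through the PlayerController, sets its lifespan, and passes on effect duration and damage per second.
; An impulse on the potion, mostly forward with a slight upward share, creates the lobbed throw.
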(event EventAction
  (params (PlayerController :type BP%20Player%20Controller%20Object%20Reference) (PlayerCharacter :type Third%20Person%20Character%20Object%20Reference))
  (bind _returnvalue (Transformation|GetActorTransform PlayerCharacter))
  (bind (_location _rotation _scale) (Math|Transform|BreakTransform _returnvalue))
  (bind _currentactor (Default|SpawnActor PlayerController "/Game/Blueprints/Spell/Poison/BP_Poison.BP_Poison_C" (Math|Transform|MakeTransform (+ (* (Transformation|GetActorForwardVector PlayerCharacter) 5e+01) _location) _rotation _scale)))
  (Actor|SetLifeSpan _currentactor (Variables|Default|GetlifeSpan))
  (bind _asbp_poison (Utilities|Casting|CastToBP_Poison _currentactor))
  (Variables|Default|SetAs%20BP%20Poison _asbp_poison)
  (Utilities|FlowControl|Sequence
    (:then_0
      (Variables|/Game/Blueprints/Spell/Poison/BP_Poison.BP_Poison_C|SetlifeSpanEffect (Variables|Default|GetAs%20BP%20Poison) (Variables|Default|GettimeEffect)))
    (:then_1
      (Variables|/Game/Blueprints/Spell/Poison/BP_Poison.BP_Poison_C|Setdammage (Variables|Default|GetAs%20BP%20Poison) (Variables|Default|GetdammagePerSec)))
    (:then_2
      (Physics|AddImpulse (Variables|/Game/Blueprints/Spell/Poison/BP_Poison.BP_Poison_C|Getpotion (Variables|Default|GetAs%20BP%20Poison)) (+ (* (Math|Vector|GetUpVector (Variables|/Game/Blueprints/Spell/Poison/BP_Poison.BP_Poison_C|Getpotion (Variables|Default|GetAs%20BP%20Poison))) (/ (Variables|Default|GetimpulseValue) 5.0)) (* (Math|Vector|GetForwardVector (Variables|/Game/Blueprints/Spell/Poison/BP_Poison.BP_Poison_C|Getpotion (Variables|Default|GetAs%20BP%20Poison))) (Variables|Default|GetimpulseValue))) "None" false))))

(fn CastSpell
  (params (PlayerController :type BP%20Player%20Controller%20Object%20Reference) (PlayerCharacter :type Third%20Person%20Character%20Object%20Reference))
  (bind _canaction_ (|CallParentFunction PlayerController PlayerCharacter))
  (if _canaction_
    (CallFunction|Action PlayerController PlayerCharacter)))