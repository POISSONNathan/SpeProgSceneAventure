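; BP_Poison is a thrown poison potion spell that applies damage over time to the first enemy it touches.
; On spawn, a physics impulse launches the potion forward and up.
; The first BP_Enemy overlap hides the potion, spawns a poison effect that follows the enemy on Tick, and starts the actor's lifespan.
; A self-calling delayed event damages the enemy every second, and the effect is removed when the spell is destroyed.
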(event OnComponentBeginOverlap(Sphere1)
  (params (OverlappedComponent :type Primitive%20Component%20Object%20Reference) (OtherActor :type Actor%20Object%20Reference) (OtherComp :type Primitive%20Component%20Object%20Reference) (OtherBodyIndex :type Integer) (bFromSweep :type Boolean) (SweepResult :type Hit%20Result%20Structure%20%28by%20ref%29))
  (if (not (Variables|Default|GethasTouch?))
    (bind _asbp_enemy (Utilities|Casting|CastToBP_Enemy OtherActor))
    (Variables|Default|SethasTouch? true)
    (Variables|Default|SetcurrentEnemy _asbp_enemy)
    (bind _returnvalue (Effects|SpawnEmitteratLocation "/Game/InfinityBladeEffects/Effects/FX_Skill_Whirlwind/P_Whirlwind_Poison_Veng_01.P_Whirlwind_Poison_Veng_01" (Transformation|GetWorldLocation (Variables|/Script/Engine.Character|GetMesh (Variables|Default|GetcurrentEnemy)))))
    (Variables|Default|SetcurrentFX _returnvalue)
    (Rendering|SetVisibility (Variables|Default|Getpotion) false false)
    (Actor|SetLifeSpan (Variables|Default|GetlifeSpanEffect))
    (Utilities|FlowControl|RetriggerableDelay 1.0)
    (CallFunction|DammagePerSec)
    (Game|AssignOnDestroyed (delegate Custom|WhenActorDestroyed))))

(event Custom|WhenActorDestroyed
  (params (DestroyedActor :type Actor%20Object%20Reference))
  (Components|DestroyComponent (Variables|Default|GetcurrentFX)))

(event Custom|DammagePerSec
  (if (Utilities|IsValid (Variables|Default|GetcurrentEnemy))
    (Default|ChangeLife (Variables|Default|GetcurrentEnemy) (Variables|Default|Getdammage))
    (Utilities|FlowControl|RetriggerableDelay 1.0)
    (CallFunction|DammagePerSec)))

(event EventTick
  (params (DeltaSeconds :type Float%20%28single-precision%29))
  (bind _currentenemy (Variables|Default|GetcurrentEnemy)
    (:then
      (Transformation|SetWorldLocation (Variables|Default|GetcurrentFX) (Transformation|GetWorldLocation (Variables|/Script/Engine.Character|GetMesh _currentenemy)) false false))
    (:else)))

(event EventBeginPlay
  (bind _potion (Variables|Default|Getpotion))
  (Physics|SetSimulatePhysics _potion true)
  (Physics|AddImpulse (Variables|Default|Getpotion) (+ (* (Math|Vector|GetUpVector _potion) 1e+03) (* (Math|Vector|GetForwardVector _potion) 5e+03)) "None" false))

(fn ConstructionScript)