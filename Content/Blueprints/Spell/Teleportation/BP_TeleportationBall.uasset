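; BP_TeleportationBall is a teleport spell projectile that moves player 0's character to wherever the ball is destroyed.
; BeginPlay binds the destroyed event and sets the current spell to DA_TeleportationSpell.
; Each tick steps the ball forward by BallSpeed without sweep or delta-time scaling, then runs a short, debug-drawn Visibility trace ahead to decide when to destroy it.
; The destroyed handler performs the teleport, so any destruction triggers it.
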(event Custom|WhenActorDestroyed
  (params (DestroyedActor :type Actor%20Object%20Reference))
  (bind _asthird_person_character (Utilities|Casting|CastToThirdPersonCharacter (Game|GetPlayerCharacter 0)))
  (Transformation|SetActorLocation _asthird_person_character (Transformation|GetActorLocation) false false))

(event EventTick
  (params (DeltaSeconds :type Float%20%28single-precision%29))
  (bind _returnvalue (Transformation|GetActorLocation))
  (Transformation|SetActorLocation (+ (Transformation|GetActorLocation) (* (Transformation|GetActorForwardVector) (Variables|Default|GetballSpeed))) false false)
  (bind _outhit (Collision|LineTraceByChannel _returnvalue (+ _returnvalue (* (Transformation|GetActorForwardVector) 75.0)) "TraceTypeQuery1" false 0 "ForDuration"))
  (if (!= (.HitActor (Collision|BreakHitResult _outhit)) 0)
    (Actor|DestroyActor)))

(event EventBeginPlay
  (Game|AssignOnDestroyed (delegate Custom|WhenActorDestroyed))
  (Variables|Default|SetcurrentSpell "/Game/Blueprints/Spell/Teleportation/DA_TeleportationSpell.DA_TeleportationSpell"))

(fn ConstructionScript)