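; Teleportation spell Blueprint that launches a teleportation ball from the player character.
; CastSpell checks the controller's Mana against ManaCost, passes the negated cost to SetMana, then fires Action and reports success.
; Action has the PlayerController spawn BP_TeleportationBall just ahead of the character with matching rotation and scale, then applies the spell's LifeSpan and BallSpeed to it.
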(event EventAction
  (params (PlayerController :type BP%20Player%20Controller%20Object%20Reference) (PlayerCharacter :type Third%20Person%20Character%20Object%20Reference))
  (bind _returnvalue (Transformation|GetActorTransform PlayerCharacter))
  (bind (_location _rotation _scale) (Math|Transform|BreakTransform _returnvalue))
  (bind _currentactor (Default|SpawnActor PlayerController "/Game/Blueprints/Spell/Teleportation/BP_TeleportationBall.BP_TeleportationBall_C" (Math|Transform|MakeTransform (+ (* (Transformation|GetActorForwardVector PlayerCharacter) 5e+01) _location) _rotation _scale)))
  (Actor|SetLifeSpan _currentactor (Variables|Default|GetlifeSpan))
  (bind _asbp_teleportation_ball (Utilities|Casting|CastToBP_TeleportationBall _currentactor))
  (Variables|/Game/Blueprints/Spell/Teleportation/BP_TeleportationBall.BP_TeleportationBall_C|SetballSpeed _asbp_teleportation_ball (Variables|Default|GetballSpeed)))

(fn CastSpell
  (params (PlayerController :type BP%20Player%20Controller%20Object%20Reference) (PlayerCharacter :type Third%20Person%20Character%20Object%20Reference))
  (if (>= (Variables|/Game/Blueprints/BP_PlayerController.BP_PlayerController_C|Getmana PlayerController) (Variables|Default|GetManaCost))
    (Default|SetMana PlayerController (* (Variables|Default|GetManaCost) -1.0))
    (CallFunction|Action PlayerController PlayerCharacter)
    (return true)))