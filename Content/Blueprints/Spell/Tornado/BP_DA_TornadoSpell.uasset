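; Tornado spell data asset Blueprint that defines how the player casts and spawns a tornado.
; Casting requires enough mana and the character moving on the ground, and triggers a long cast animation on the controller.
; Its action spawns BP_Tornado below the character through the controller, then passes in lifespan, particle template, damage and speed.
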(event EventAction
  (params (PlayerController :type BP%20Player%20Controller%20Object%20Reference) (PlayerCharacter :type Third%20Person%20Character%20Object%20Reference))
  (bind _returnvalue (Transformation|GetActorTransform PlayerCharacter))
  (bind (_location _rotation _scale) (Math|Transform|BreakTransform _returnvalue))
  (bind _currentactor (Default|SpawnActor PlayerController "/Game/Blueprints/Spell/Tornado/BP_Tornado.BP_Tornado_C" (Math|Transform|MakeTransform (+ _location "0, 0,-100.000000") _rotation _scale)))
  (bind _asbp_tornado (Utilities|Casting|CastToBP_Tornado _currentactor))
  (Actor|SetLifeSpan _asbp_tornado (Variables|Default|GetlifeSpan))
  (Effects|Components|ParticleSystem|SetTemplate (Variables|/Game/Blueprints/Spell/Tornado/BP_Tornado.BP_Tornado_C|GetParticleSystem _asbp_tornado) (Variables|Default|GetparticleSystemUse))
  (Utilities|FlowControl|Sequence
    (:then_0
      (Variables|/Game/Blueprints/Spell/Tornado/BP_Tornado.BP_Tornado_C|Setdammage _asbp_tornado (Variables|Default|Getdammage)))
    (:then_1
      (Variables|/Game/Blueprints/Spell/Tornado/BP_Tornado.BP_Tornado_C|Setspeed _asbp_tornado (Variables|Default|Getspeed)))))

(fn AdditionalEffect
  (params (PlayerController :type BP%20Player%20Controller%20Object%20Reference) (PlayerCharaacter :type Third%20Person%20Character%20Object%20Reference))
  (Default|LongAnimCastSpell PlayerController self)
  (Variables|/Game/Blueprints/BP_PlayerController.BP_PlayerController_C|SetinSpellAnimation PlayerController true))

(fn ConditiontoCast
  (params (PlayerController :type BP%20Player%20Controller%20Object%20Reference) (PlayerCharacter :type Third%20Person%20Character%20Object%20Reference))
  (return (and (>= (Variables|/Game/Blueprints/BP_PlayerController.BP_PlayerController_C|Getmana PlayerController) (Variables|Default|GetManaCost)) (AI|Components|NavMovement|IsMovingonGround (Variables|/Script/Engine.Character|GetCharacterMovement PlayerCharacter)))))