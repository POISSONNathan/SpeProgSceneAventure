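; BP_Tornado is a tornado spell actor that flies forward until it catches an enemy, then sticks to it and damages it.
; Each tick it moves along its forward vector by Speed, unscaled by delta time.
; A BP_Enemy overlapping the box collider becomes the target, so the tornado snaps to its mesh and calls ChangeLife every tick.
; Forward travel resumes once that enemy is no longer valid.
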(event OnComponentBeginOverlap(BoxCollider)
  (params (OverlappedComponent :type Primitive%20Component%20Object%20Reference) (OtherActor :type Actor%20Object%20Reference) (OtherComp :type Primitive%20Component%20Object%20Reference) (OtherBodyIndex :type Integer) (bFromSweep :type Boolean) (SweepResult :type Hit%20Result%20Structure%20%28by%20ref%29))
  (bind _asbp_enemy (Utilities|Casting|CastToBP_Enemy OtherActor))
  (Variables|Default|SetcurrentEnemy _asbp_enemy)
  (Variables|Default|SetenemyTag true))

(event EventTick
  (params (DeltaSeconds :type Float%20%28single-precision%29))
  (if (Variables|Default|GetenemyTag)
    (bind _currentenemy (Variables|Default|GetcurrentEnemy)
      (:then
        (Transformation|SetActorLocation (Transformation|GetWorldLocation (Variables|/Script/Engine.Character|GetMesh _currentenemy)) false false)
        (bind _currentenemy_2 (Variables|Default|GetcurrentEnemy)
          (:then
            (Default|ChangeLife _currentenemy_2 (Variables|Default|Getdammage))
            (Variables|Default|GetcurrentEnemy
              (:then)
              (:else
                (Variables|Default|SetenemyTag false))))
          (:else)))
      (:else
        (Variables|Default|SetenemyTag false)))
    (else
      (Transformation|SetActorLocation (+ (Transformation|GetActorLocation) (* (Transformation|GetActorForwardVector) (Variables|Default|Getspeed))) false false))))

(fn ConstructionScript)